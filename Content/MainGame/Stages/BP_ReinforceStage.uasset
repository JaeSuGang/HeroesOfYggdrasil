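; BP_ReinforceStage is a game stage that brings in enemy reinforcements and is meant to end on a timer.
; On entry it enables a 20-second timer and calls TestSpawner, which reads the Minion_Archer data table row to create a small delayed spawner at a hardcoded location.
; ShouldEnterNextStage returns true once Timer runs out.
; Tick and exit do nothing, so this graph never decrements Timer itself.
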(event `self.OnEnterStage`
  (set `self.bIsTimerEnabled` true)
  (set `self.Timer` 20.0)
  (bind _returnvalue (`|GetDataTableRow` "/Game/Data/EnemyBaseStatusDataTable.EnemyBaseStatusDataTable" "Minion_Archer")
    (:`then`
      (`self.SpawnEnemySpawner` _returnvalue (350.0 -3000.0 300.0) 3 1.0))))

(event `self.OnExitStage`)

(event `self.ReceiveTick`
  (params (DeltaSeconds :type "Float (single-precision)"))
  (if true
    _))

(fn `ShouldEnterNextStage`
  (returns (ReturnValue :type Boolean))
  (if (<= (`self.Timer`) 0.0)
    (return true)
    (else
      (return false))))

(fn `UserConstructionScript`)